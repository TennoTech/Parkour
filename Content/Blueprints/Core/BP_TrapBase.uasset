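; BP_TrapBase is a trap actor that damages BP_Player inside its collision box.
; On overlap it applies InitialDamage through the player's health component, then a looping one-second timer applies DamagePerSecond until the player leaves.
; At BeginPlay, IsInstaKill replaces InitialDamage with a class default from ACP_Health.
; The construction script sizes the box from variables and toggles its in-game visibility for debugging.
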(event OnComponentBeginOverlap(TrapCollision)
  (params (OverlappedComponent :type Primitive%20Component%20Object%20Reference) (OtherActor :type Actor%20Object%20Reference) (OtherComp :type Primitive%20Component%20Object%20Reference) (OtherBodyIndex :type Integer) (bFromSweep :type Boolean) (SweepResult :type Hit%20Result%20Structure%20%28by%20ref%29))
  (bind _asbp_player (Utilities|Casting|CastToBP_Player OtherActor))
  (Utilities|IsValid (Variables|Default|GetPlayerRef)
    (:Is%20Valid
      _)
    (:Is%20Not%20Valid
      (bind _output_get (Variables|Default|SetPlayerRef _asbp_player))))
  (Default|DamageHealth (Variables|/Game/Blueprints/Player/BP_Player.BP_Player_C|GetACP_Health _output_get) (Variables|Default|GetInitialDamage))
  (CallFunction|StartTrapSequence))

(event OnComponentEndOverlap(TrapCollision)
  (params (OverlappedComponent :type Primitive%20Component%20Object%20Reference) (OtherActor :type Actor%20Object%20Reference) (OtherComp :type Primitive%20Component%20Object%20Reference) (OtherBodyIndex :type Integer))
  (Utilities|Casting|CastToBP_Player OtherActor)
  (Utilities|IsValid (Variables|Default|GetPlayerRef)
    (:Is%20Valid
      (Variables|Default|SetPlayerRef 0))
    (:Is%20Not%20Valid
      _))
  (CallFunction|EndTrapSequence))

(event Custom|DamagePlayer_Event
  (bind _playerref (Variables|Default|GetPlayerRef))
  (Utilities|IsValid _playerref
    (:Is%20Valid
      (Default|DamageHealth (Variables|/Game/Blueprints/Player/BP_Player.BP_Player_C|GetACP_Health _playerref) (Variables|Default|GetDamagePerSecond)))
    (:Is%20Not%20Valid
      (Utilities|Time|InvalidateTimerHandle (Variables|Default|GetDamageTimerHandle)))))

(event Custom|EndTrapSequence
  (bind _damagetimerhandle (Variables|Default|GetDamageTimerHandle))
  (if (Utilities|Time|IsValidTimerHandle _damagetimerhandle)
    (Utilities|Time|InvalidateTimerHandle _damagetimerhandle)
    (else
      (Development|PrintString "Invalid: Timer Handle"))))

(event Custom|StartTrapSequence
  (bind _returnvalue (Utilities|Time|SetTimerbyEvent (delegate Custom|DamagePlayer_Event) 1.0 true))
  (Variables|Default|SetDamageTimerHandle _returnvalue))

(event EventBeginPlay
  (if (Variables|Default|GetIsInstaKill?)
    (Variables|Default|SetInitialDamage (Utilities|GetClassDefaults "/Game/Blueprints/ACP_Health.ACP_Health_C"))))

(fn ConstructionScript
  (Components|Box|SetBoxExtent (Variables|Default|GetTrapCollision) (Math|Vector|MakeVector (Variables|Default|GetCollisionAxisX) (Variables|Default|GetCollisionAxisY) (Variables|Default|GetCollisionHeight)) true)
  (Development|SetHiddeninGame (Variables|Default|GetTrapCollision) (not (Variables|Default|GetEnableDebugCollision)) false))