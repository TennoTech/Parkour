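; BP_GameMode is a game mode that tracks the game-over state and handles the end of a failed level.
; It caches the player character on BeginPlay and exposes a setter and getter for the IsGameOver flag.
; SetCompletedState triggers EndGame, which, if the flag is true, disables player input and shows WBP_LevelInfo with IsLevelCompleted always false, despite the setter's name.
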(event Custom|EndGame
  (if (Variables|Default|GetIsGameOver)
    (Input|DisableInput (Variables|Default|GetPlayerRef) (Game|GetPlayerController 0))
    (bind _returnvalue (UserInterface|CreateWidget "/Game/Blueprints/Widgets/Gameplay/WBP_LevelInfo.WBP_LevelInfo_C"))
    (UserInterface|Viewport|AddtoViewport _returnvalue 0)))

(event EventBeginPlay
  (bind _asbp_player (Utilities|GetPlayerCharacter)
    (:then
      (Variables|Default|SetPlayerRef _asbp_player))))

(fn ConstructionScript)

(fn SetCompletedState
  (params (IsGameOver :type Boolean))
  (Variables|Default|SetIsGameOver IsGameOver)
  (CallFunction|EndGame))

(fn GetCompletedState
  (return (Variables|Default|GetIsGameOver)))