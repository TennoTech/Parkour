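; First-person player character with wall running, air-steerable multi-jump, and walk, jog, sprint and crouch movement.
; Capsule hits on steep surfaces start wall runs, which disable gravity, tilt the camera and re-trace the wall through a timeline until input or wall is lost.
; Input flags resolve one movement state, driving timelines for speed blending and crouch height, with a trace blocking standing under obstacles.
; Tick caps horizontal air speed.
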(event OnComponentHit(CapsuleComponent)
  (params (HitComponent :type Primitive%20Component%20Object%20Reference) (OtherActor :type Actor%20Object%20Reference) (OtherComp :type Primitive%20Component%20Object%20Reference) (NormalImpulse :type Vector :default "0, 0, 0") (Hit :type Hit%20Result%20Structure%20%28by%20ref%29))
  (bind _impactnormal (Collision|BreakHitResult Hit))
  (bind (_direction _side) (WallRunning|FindRunDirectionandSide _impactnormal))
  (Utilities|OnWall
    (:false
      (if (WallRunning|CanSurfacebeWallRan _impactnormal)
        (if (AI|Components|NavMovement|IsFalling (Variables|Character|GetCharacterMovement))
          (Variables|WallRunning|SetWallRunDirection _direction)
          (Variables|WallRunning|SetWallRunSide _side)
          (if (WallRunning|AreRequiredKeysDown)
            (CallFunction|BeginWallRun)))))))

(event Custom|ChangeMovementSpeed
  (Timeline|SpeedTransitionTimeline PlayFromStart
    (:Update
      (Variables|/Script/Engine.CharacterMovementComponent|SetMaxWalkSpeed (Variables|Character|GetCharacterMovement) (Math|Float|Lerp (Math|Vector|VectorLength (Transformation|GetVelocity)) (Variables|Default|GetTargetMovementSpeed) 0.1)))))

(event Custom|EndWallRun
  (params (Reason :type E_WallRunEndReason%20Enum :default "NewEnumerator0"))
  (bind _charactermovement (Variables|Character|GetCharacterMovement))
  (CallFunction|ResetJump (Utilities|Select :Index Reason :NewEnumerator0 2 :NewEnumerator1 (Variables|WallRunning|GetMaxJumps)))
  (Variables|/Script/Engine.CharacterMovementComponent|SetAirControl _charactermovement 0.05)
  (Variables|/Script/Engine.CharacterMovementComponent|SetGravityScale _charactermovement 1.0)
  (Class|MovementComponent|SetPlaneConstraintNormal _charactermovement "0, 0, 0")
  (Variables|WallRunning|SetisWallRunning false)
  (CallFunction|EndCameraTilt)
  (Timeline|WallRunTimeline Stop
    (:Update
      (WallRunning|UpdateWallRun))))

(event Custom|BeginWallRun
  (bind _charactermovement (Variables|Character|GetCharacterMovement))
  (Variables|/Script/Engine.CharacterMovementComponent|SetAirControl _charactermovement 0.0)
  (Variables|/Script/Engine.CharacterMovementComponent|SetGravityScale _charactermovement 0.0)
  (Class|MovementComponent|SetPlaneConstraintNormal _charactermovement "0,0.000000,1.000000")
  (Variables|WallRunning|SetisWallRunning true)
  (CallFunction|BeginCameraTilt)
  (Timeline|WallRunTimeline Play
    (:Update
      (WallRunning|UpdateWallRun))))

(event Custom|EndCrouch
  (bind _standingcapsulecapheight (Variables|Default|GetStandingCapsuleCapHeight))
  (bind _camera (Variables|Default|GetCamera))
  (bind _relativelocation (Variables|/Script/Engine.SceneComponent|GetRelativeLocation _camera))
  (bind _animtrack (Timeline|CrouchTimeline Reverse)
    (:Update
      (Components|Capsule|SetCapsuleHalfHeight (Variables|Collision|GetCapsuleComponent) (Math|Float|MapRangeClamped _animtrack 0.0 1.0 (/ _standingcapsulecapheight 1.5) _standingcapsulecapheight) true)
      (Transformation|SetRelativeLocation _camera (Math|Vector|MakeVector (.x _relativelocation) (.y _relativelocation) (Math|Float|MapRangeClamped _animtrack 0.0 1.0 25.0 (Variables|Default|GetStandingCameraZOffset))) false false))))

(event Custom|EndCameraTilt
  (bind _returnvalue (Pawn|GetController))
  (bind _returnvalue_2 (Pawn|GetControlRotation _returnvalue :!class /Script/Engine.Controller))
  (bind _cameraroll (Timeline|CameraTiltTimeline Reverse)
    (:Update
      (Pawn|SetControlRotation _returnvalue (Math|Rotator|MakeRotator (* _cameraroll (Utilities|Select :Index (Variables|WallRunning|GetWallRunSide) :NewEnumerator0 1.0 :NewEnumerator1 -1.0)) (.pitch _returnvalue_2) (.yaw _returnvalue_2))))))

(event Custom|BeginCameraTilt
  (bind _returnvalue (Pawn|GetController))
  (bind _returnvalue_2 (Pawn|GetControlRotation _returnvalue :!class /Script/Engine.Controller))
  (bind _cameraroll (Timeline|CameraTiltTimeline Play)
    (:Update
      (Pawn|SetControlRotation _returnvalue (Math|Rotator|MakeRotator (* _cameraroll (Utilities|Select :Index (Variables|WallRunning|GetWallRunSide) :NewEnumerator0 1.0 :NewEnumerator1 -1.0)) (.pitch _returnvalue_2) (.yaw _returnvalue_2))))))

(event Custom|BeginCrouch
  (bind _standingcapsulecapheight (Variables|Default|GetStandingCapsuleCapHeight))
  (bind _camera (Variables|Default|GetCamera))
  (bind _relativelocation (Variables|/Script/Engine.SceneComponent|GetRelativeLocation _camera))
  (bind _animtrack (Timeline|CrouchTimeline Play)
    (:Update
      (Components|Capsule|SetCapsuleHalfHeight (Variables|Collision|GetCapsuleComponent) (Math|Float|MapRangeClamped _animtrack 0.0 1.0 (/ _standingcapsulecapheight 1.5) _standingcapsulecapheight) true)
      (Transformation|SetRelativeLocation _camera (Math|Vector|MakeVector (.x _relativelocation) (.y _relativelocation) (Math|Float|MapRangeClamped _animtrack 0.0 1.0 25.0 (Variables|Default|GetStandingCameraZOffset))) false false))))

(event EventBeginPlay
  (CallFunction|ResetJump (Variables|WallRunning|GetMaxJumps))
  (Class|MovementComponent|SetPlaneConstraintEnabled (Variables|Character|GetCharacterMovement) true)
  (CallFunction|InitializeMovementSpeed)
  (Variables|Default|SetStandingCameraZOffset (.z (Variables|/Script/Engine.SceneComponent|GetRelativeLocation (Variables|Default|GetCamera))))
  (Variables|Default|SetStandingCapsuleCapHeight (Components|Capsule|GetScaledCapsuleHalfHeight (Variables|Collision|GetCapsuleComponent))))

(event EventTick
  (params (DeltaSeconds :type Float%20%28single-precision%29))
  (WallRunning|ClampHorizontalVelocity)
  (Utilities|SwitchMovementState
    (:Crouch
      (if (Movement|CanStand)
        (CallFunction|ResolveMovementState)))))

(event Custom|ResetJump
  (params (Jumps :type Integer))
  (Variables|WallRunning|SetJumpsLeft (Math|Integer|Clamp(Integer) Jumps 0 (Variables|WallRunning|GetMaxJumps))))

(event EventOnLanded
  (params (Hit :type Hit%20Result%20Structure%20%28by%20ref%29))
  (CallFunction|ResetJump (Variables|WallRunning|GetMaxJumps))
  (Variables|Default|SetLocomotionState "NewEnumerator5"))

(event Input|ActionEvents|InputActionJump
  (params (Key :type Key%20Structure :default "None"))
  (:Pressed
    (Variables|Default|SetLocomotionState "NewEnumerator6")
    (Utilities|ConsumeJump
      (:Consumed
        (Character|LaunchCharacter (WallRunning|FindLaunchVelocity) false true)
        (Utilities|OnWall
          (:true
            (CallFunction|EndWallRun "NewEnumerator1"))))))
  (:Released
    (Character|StopJumping)))

(event Input|ActionEvents|InputActionCrouch
  (params (Key :type Key%20Structure :default "None"))
  (:Pressed
    (Variables|Default|SetIsCrouchKeyDown true)
    (Utilities|SwitchMovementState
      (:Walk
        _)
      (:Jog
        _))
    (CallFunction|SetMovementState "NewEnumerator7"))
  (:Released
    (Variables|Default|SetIsCrouchKeyDown false)
    (CallFunction|ResolveMovementState)))

(event Input|ActionEvents|InputActionSprint
  (params (Key :type Key%20Structure :default "None"))
  (:Pressed
    (Variables|Default|SetIsSprintKeyDown true)
    (Variables|Default|SetIsWalkKeyDown false)
    (Utilities|SwitchMovementState
      (:Walk
        _)
      (:Jog
        _)
      (:Crouch
        _))
    (CallFunction|ResolveMovementState))
  (:Released
    (Variables|Default|SetIsSprintKeyDown false)
    (Utilities|SwitchMovementState
      (:Sprint
        (CallFunction|ResolveMovementState)))))

(event Input|ActionEvents|InputActionWalk
  (params (Key :type Key%20Structure :default "None"))
  (:Pressed
    (if (Variables|Default|GetIsWalkKeyDown)
      (Variables|Default|SetIsWalkKeyDown false)
      (else
        (Variables|Default|SetIsWalkKeyDown true)))
    (CallFunction|ResolveMovementState)))

(event Input|AxisEvents|InputAxisMoveForward
  (params (AxisValue :type Float%20%28single-precision%29))
  (bind _output_get (Variables|WallRunning|SetForwardAxis AxisValue))
  (Pawn|Input|AddMovementInput (Math|Vector|GetForwardVector (Variables|Collision|GetCapsuleComponent)) _output_get false))

(event Input|AxisEvents|InputAxisMoveRight
  (params (AxisValue :type Float%20%28single-precision%29))
  (bind _output_get (Variables|WallRunning|SetRightAxis AxisValue))
  (Pawn|Input|AddMovementInput (Math|Vector|GetRightVector (Variables|Collision|GetCapsuleComponent)) _output_get false))

(event Input|AxisEvents|InputAxisTurn
  (params (AxisValue :type Float%20%28single-precision%29))
  (Pawn|Input|AddControllerYawInput AxisValue))

(event Input|AxisEvents|InputAxisLookUp
  (params (AxisValue :type Float%20%28single-precision%29))
  (Pawn|Input|AddControllerPitchInput AxisValue))

(fn ConstructionScript)

(fn FindRunDirectionandSide
  (params (WallNormal :type Vector))
  (bind _output_get (LocalVariables|SetLocalSide (select (> (Math|Vector2D|DotProduct(2D) (Math|Conversions|ToVector2D(Vector) WallNormal) (Math|Conversions|ToVector2D(Vector) (Transformation|GetActorRightVector))) 0.0) "NewEnumerator0" "NewEnumerator1")))
  (return (Math|Vector|CrossProduct WallNormal (Utilities|Select :Index _output_get :NewEnumerator0 "0.000000, 0,-1.000000" :NewEnumerator1 "0,0.000000,1.000000")) (LocalVariables|GetLocalSide)))

(fn CanSurfacebeWallRan
  (params (SurfaceNormal :type Vector))
  (bind (_x _y _z) (Math|Vector|BreakVector SurfaceNormal))
  (if (< _z -0.05)
    (return false)
    (else
      (return (< (Class|KismetMathLibrary|DegAcos (Math|Vector|DotProduct (Math|Vector|Normalize (Math|Vector|MakeVector _x _y 0.0)) SurfaceNormal)) (Class|CharacterMovementComponent|GetWalkableFloorAngle (Variables|Character|GetCharacterMovement)))))))

(fn FindLaunchVelocity
  (Utilities|FlowControl|Sequence
    (:then_0
      (if (Variables|WallRunning|GetisWallRunning)
        (LocalVariables|SetLaunchDirection (Math|Vector|CrossProduct (Variables|WallRunning|GetWallRunDirection) (Utilities|Select :Index (Variables|WallRunning|GetWallRunSide) :NewEnumerator0 "0, 0,1.000000" :NewEnumerator1 "0.000000, 0,-1.000000")))
        (elif (AI|Components|NavMovement|IsFalling (Variables|Character|GetCharacterMovement))
          (LocalVariables|SetLaunchDirection (+ (* (Transformation|GetActorRightVector) (Variables|WallRunning|GetRightAxis)) (* (Transformation|GetActorForwardVector) (Variables|WallRunning|GetForwardAxis)))))))
    (:then_1
      (return (* (+ (LocalVariables|GetLaunchDirection) "0, 0,1.000000") (Variables|/Script/Engine.CharacterMovementComponent|GetJumpZVelocity (Variables|Character|GetCharacterMovement)))))))

(fn AreRequiredKeysDown
  (if (> (Variables|WallRunning|GetForwardAxis) 0.1)
    (switch Utilities|FlowControl|Switch|SwitchonE_WallRunSide (Variables|WallRunning|GetWallRunSide)
      (:NewEnumerator0
        (return (< (Variables|WallRunning|GetRightAxis) -0.1)))
      (:NewEnumerator1
        (return (> (Variables|WallRunning|GetRightAxis) 0.1))))
    (else
      (return false))))

(fn GetHorizontalVelocity
  (return (Math|Conversions|ToVector2D(Vector) (Variables|/Script/Engine.MovementComponent|GetVelocity (Variables|Character|GetCharacterMovement)))))

(fn SetHorizontalVelocity
  (params (HorizontalVelocity :type Vector%202D%20Structure))
  (bind _charactermovement (Variables|Character|GetCharacterMovement))
  (Variables|/Script/Engine.MovementComponent|SetVelocity _charactermovement (Math|Vector|MakeVector (.x HorizontalVelocity) (.y HorizontalVelocity) (.z (Variables|/Script/Engine.MovementComponent|GetVelocity _charactermovement)))))

(fn UpdateWallRun
  (bind _returnvalue (Transformation|GetActorLocation))
  (bind _charactermovement (Variables|Character|GetCharacterMovement))
  (if (WallRunning|AreRequiredKeysDown)
    (bind (_outhit _returnvalue_2) (Collision|LineTraceByChannel _returnvalue (+ _returnvalue (* (Math|Vector|CrossProduct (Variables|WallRunning|GetWallRunDirection) (Utilities|Select :Index (Variables|WallRunning|GetWallRunSide) :NewEnumerator0 "0, 0,-1.000000" :NewEnumerator1 "0,0.000000,1.000000")) 1e+02)) "TraceTypeQuery1" false 0 "None"))
    (if _returnvalue_2
      (if (Utilities|Enum|Equal(Enum) (.Side (WallRunning|FindRunDirectionandSide (.ImpactNormal (Collision|BreakHitResult _outhit)))) (Variables|WallRunning|GetWallRunSide))
        (bind _output_get (Variables|WallRunning|SetWallRunDirection (.Direction (WallRunning|FindRunDirectionandSide (.ImpactNormal (Collision|BreakHitResult _outhit)))))) ; getting wall direction\nIE: wall has changed directions
        (Variables|/Script/Engine.MovementComponent|SetVelocity _charactermovement (Math|Vector|MakeVector (.x (* (* _output_get (Class|MovementComponent|GetModifiedMaxSpeed _charactermovement)) -1.0)) (.y (* (* _output_get (Class|MovementComponent|GetModifiedMaxSpeed _charactermovement)) -1.0)) 0.0)) ; update velocity to accomodate\nif walls change mid wall run
        (else
          (CallFunction|EndWallRun "NewEnumerator0")))
      (else
        (CallFunction|EndWallRun "NewEnumerator0")))
    (else
      (CallFunction|EndWallRun "NewEnumerator0"))))

(fn ClampHorizontalVelocity
  (bind _returnvalue (WallRunning|GetHorizontalVelocity))
  (bind _charactermovement (Variables|Character|GetCharacterMovement))
  (bind _returnvalue_2 (Math|Vector2D|Vector2DLength _returnvalue))
  (bind _returnvalue_3 (Class|MovementComponent|GetModifiedMaxSpeed _charactermovement))
  (bind _returnvalue_4 (/ _returnvalue_2 _returnvalue_3))
  (if (AI|Components|NavMovement|IsFalling (Variables|Character|GetCharacterMovement))
    (if (Utilities|Enum|Equal(Enum) (Variables|Default|GetLocomotionState) "NewEnumerator7")
      (Variables|Default|SetLocomotionState "NewEnumerator7")
      (else
        (Variables|Default|SetLocomotionState "NewEnumerator6")
        (if (> _returnvalue_4 1.0) ; moving to quickly
          (WallRunning|SetHorizontalVelocity (/ (WallRunning|GetHorizontalVelocity) _returnvalue_4)))))))

(fn CanStand
  (bind _returnvalue (Transformation|GetActorLocation))
  (bind _capsulecomponent (Variables|Collision|GetCapsuleComponent))
  (bind _returnvalue_2 (Components|Capsule|GetScaledCapsuleHalfHeight _capsulecomponent))
  (bind _returnvalue_3 (- _returnvalue (Math|Vector|MakeVector 0.0 0.0 _returnvalue_2)))
  (if (Variables|Default|GetIsCrouchKeyDown)
    (return false)
    (else
      (bind _returnvalue_4 (Collision|LineTraceByChannel _returnvalue_3 (+ _returnvalue_3 (Math|Vector|MakeVector 0.0 0.0 (* (Variables|Default|GetStandingCapsuleCapHeight) 2.0))) "TraceTypeQuery1" false 0 "None"))
      (return (not _returnvalue_4)))))

(fn CanJog
  (return (and (Movement|CanStand) (not (Variables|Default|GetIsWalkKeyDown)))))

(fn CanWalk
  (return (and (Movement|CanStand) (Variables|Default|GetIsWalkKeyDown))))

(fn CanSprint
  (if (Variables|Default|GetIsSprintKeyDown)
    (return (Movement|CanStand))
    (else
      (return false))))

(fn ResolveMovementState
  (CallFunction|SetMovementState (select (Variables|Default|GetIsCrouchKeyDown) "NewEnumerator7" (select (Movement|CanSprint) "NewEnumerator5" (select (Movement|CanJog) "NewEnumerator2" (select (Movement|CanWalk) "NewEnumerator1" "NewEnumerator7"))))))

(fn SetMovementState
  (params (NewMovementState :type E_MovementState%20Enum :default "NewEnumerator1"))
  (if (Utilities|Enum|NotEqual(Enum) NewMovementState (Variables|Default|GetMovementState))
    (LocalVariables|SetPrevMovementState (Variables|Default|GetMovementState))
    (Variables|Default|SetMovementState NewMovementState)
    (CallFunction|OnMovementStateChanged (LocalVariables|GetPrevMovementState))
    (Utilities|SwitchMovementState
      (:Walk
        (CallFunction|EndCrouch :!label _label))
      (:Jog
        (goto _label))
      (:Sprint
        (goto _label))
      (:Crouch
        (CallFunction|BeginCrouch)))))

(fn OnMovementStateChanged
  (params (PrevMovementState :type E_MovementState%20Enum :default "NewEnumerator1"))
  (Utilities|FlowControl|Sequence
    (:then_0
      (Variables|Default|SetTargetMovementSpeed (Utilities|Select :Index (Variables|Default|GetMovementState) :NewEnumerator1 (Variables|Default|GetWalkSpeed) :NewEnumerator2 (Variables|Default|GetJogSpeed) :NewEnumerator5 (Variables|Default|GetSprintSpeed) :NewEnumerator7 (Variables|Default|GetCrouchSpeed)))
      (CallFunction|ChangeMovementSpeed))))

(fn InitializeMovementSpeed
  (bind _output_get (Variables|Default|SetJogSpeed (select (== (Variables|Default|GetJogSpeed) 0.0) (Variables|/Script/Engine.CharacterMovementComponent|GetMaxWalkSpeed (Variables|Character|GetCharacterMovement)) (Variables|Default|GetJogSpeed))))
  (bind _output_get_2 (Variables|/Script/Engine.CharacterMovementComponent|SetMaxWalkSpeed (Variables|Character|GetCharacterMovement) _output_get))
  (bind _output_get_3 (Variables|Default|SetTargetMovementSpeed _output_get_2))
  (Variables|Default|SetSprintSpeed (select (== (Variables|Default|GetSprintSpeed) 0.0) (* _output_get_3 2.0) (Variables|Default|GetSprintSpeed)))
  (Variables|Default|SetWalkSpeed (select (== (Variables|Default|GetWalkSpeed) 0.0) (/ (Variables|Default|GetTargetMovementSpeed) 2.0) (Variables|Default|GetWalkSpeed)))
  (Variables|Default|SetCrouchSpeed (select (== (Variables|Default|GetCrouchSpeed) 0.0) (/ (Variables|Default|GetTargetMovementSpeed) 1.75) (Variables|Default|GetCrouchSpeed))))