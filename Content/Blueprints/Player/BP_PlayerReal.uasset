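; First-person player character with walk, sprint, crouch, slide, limited-count jumps and wall running, plus a debug UI widget.
; Inputs drive movement and locomotion state machines that set speed, friction and capsule height, with timelines easing transitions and camera roll.
; Capsule hits start wall runs, which disable gravity and re-trace the wall each update to follow it.
; Slides apply slope-based force from the floor normal, capped at sprint speed.
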(event OnComponentHit(CapsuleComponent)
  (params (HitComponent :type Primitive%20Component%20Object%20Reference) (OtherActor :type Actor%20Object%20Reference) (OtherComp :type Primitive%20Component%20Object%20Reference) (NormalImpulse :type Vector :default "0, 0, 0") (Hit :type Hit%20Result%20Structure%20%28by%20ref%29))
  (bind _impactnormal (Collision|BreakHitResult Hit))
  (bind (_direction _side) (WallRunning|FindRunDirectionandSide _impactnormal))
  (Utilities|OnWall
    (:false
      (if (WallRunning|CanSurfacebeWallRan _impactnormal)
        (if (AI|Components|NavMovement|IsFalling (Variables|Character|GetCharacterMovement))
          (Variables|WallRunning|SetWallRunDirection _direction)
          (Variables|WallRunning|SetWallRunSide _side)
          (if (WallRunning|AreRequiredKeysDown)
            (CallFunction|BeginWallRun)))))))

(event Custom|EndWallRun
  (params (Reason :type E_WallRunEndReason%20Enum :default "NewEnumerator0"))
  (bind _charactermovement (Variables|Character|GetCharacterMovement))
  (bind _maxjumps (Variables|WallRunning|GetMaxJumps))
  (Character|LaunchCharacter (WallRunning|FindLaunchVelocity) false true)
  (if (Variables|Debug|GetEnableDoubleJump)
    (CallFunction|ResetJump (Utilities|Select :Index Reason :NewEnumerator0 _maxjumps :NewEnumerator1 _maxjumps)))
  (Variables|/Script/Engine.CharacterMovementComponent|SetAirControl _charactermovement 0.05)
  (Variables|/Script/Engine.CharacterMovementComponent|SetGravityScale _charactermovement 1.0)
  (Class|MovementComponent|SetPlaneConstraintNormal _charactermovement "0, 0, 0")
  (Variables|WallRunning|SetisWallRunning false)
  (CallFunction|EndCameraTilt)
  (Timeline|WallRunTimeline Stop
    (:Update
      (WallRunning|UpdateWallRun))))

(event Custom|BeginSlideCameraTilt
  (bind _returnvalue (Game|GetPlayerController 0))
  (bind _returnvalue_2 (Pawn|GetControlRotation _returnvalue :!class /Script/Engine.Controller))
  (bind _tiltvalue (Timeline|SlideCameraTiltTimeline Play)
    (:Update
      (Pawn|SetControlRotation _returnvalue (Math|Rotator|MakeRotator _tiltvalue (.pitch _returnvalue_2) (.yaw _returnvalue_2))))))

(event Custom|EndSlideCameraTilt
  (bind _returnvalue (Game|GetPlayerController 0))
  (bind _returnvalue_2 (Pawn|GetControlRotation _returnvalue :!class /Script/Engine.Controller))
  (bind _tiltvalue (Timeline|SlideCameraTiltTimeline Reverse)
    (:Update
      (Pawn|SetControlRotation _returnvalue (Math|Rotator|MakeRotator _tiltvalue (.pitch _returnvalue_2) (.yaw _returnvalue_2))))))

(event Custom|ChangeMovementSpeed
  (bind _newtrack_0 (Timeline|SpeedTransitionTimeline PlayFromStart)
    (:Update
      (Variables|/Script/Engine.CharacterMovementComponent|SetMaxWalkSpeed (Variables|Character|GetCharacterMovement) (Math|Float|Lerp (Math|Vector|VectorLength (Transformation|GetVelocity)) (Variables|Movement|GetTargetMovementSpeed) _newtrack_0)))))

(event Custom|BeginWallRun
  (bind _charactermovement (Variables|Character|GetCharacterMovement))
  (Variables|/Script/Engine.CharacterMovementComponent|SetAirControl _charactermovement 0.0)
  (Variables|/Script/Engine.CharacterMovementComponent|SetGravityScale _charactermovement 0.0)
  (Class|MovementComponent|SetPlaneConstraintNormal _charactermovement "0,0.000000,1.000000")
  (Variables|WallRunning|SetisWallRunning true)
  (CallFunction|BeginCameraTilt)
  (Timeline|WallRunTimeline Play
    (:Update
      (WallRunning|UpdateWallRun))))

(event Custom|EndSlide
  (Variables|Default|SetIsSliding false)
  (CallFunction|EndSlideCameraTilt)
  (Timeline|SlideTimeline Stop
    (:Update
      (Physics|AddForce (Variables|Character|GetCharacterMovement) (Sliding|CalculateFloorInfluence (.Normal (Collision|BreakHitResult (.HitResult (Utilities|Struct|BreakFindFloorResult (Variables|/Script/Engine.CharacterMovementComponent|GetCurrentFloor (Variables|Character|GetCharacterMovement))))))))
      (Utilities|FlowControl|Sequence
        (:then_0
          (if (> (Math|Vector|VectorLength (Transformation|GetVelocity)) (Variables|Movement|GetSprintSpeed))
            (Variables|/Script/Engine.MovementComponent|SetVelocity (Variables|Character|GetCharacterMovement) (* (Math|Vector|Normalize (Transformation|GetVelocity)) (Variables|Movement|GetSprintSpeed)))))
        (:then_1
          (if (not (Variables|Default|GetIsCrouchKeyDown))
            (CallFunction|ResolveMovementState)))
        (:then_2
          (if (< (Math|Vector|VectorLength (Transformation|GetVelocity)) (Variables|Movement|GetCrouchSpeed))
            (CallFunction|ResolveMovementState)))))))

(event Custom|EndCameraTilt
  (bind _returnvalue (Pawn|GetController))
  (bind _returnvalue_2 (Pawn|GetControlRotation _returnvalue :!class /Script/Engine.Controller))
  (bind _cameraroll (Timeline|CameraTiltTimeline Reverse)
    (:Update
      (Pawn|SetControlRotation _returnvalue (Math|Rotator|MakeRotator (* _cameraroll (Utilities|Select :Index (Variables|WallRunning|GetWallRunSide) :NewEnumerator0 1.0 :NewEnumerator1 -1.0)) (.pitch _returnvalue_2) (.yaw _returnvalue_2))))))

(event Custom|BeginCameraTilt
  (bind _returnvalue (Pawn|GetController))
  (bind _returnvalue_2 (Pawn|GetControlRotation _returnvalue :!class /Script/Engine.Controller))
  (bind _cameraroll (Timeline|CameraTiltTimeline Play)
    (:Update
      (Pawn|SetControlRotation _returnvalue (Math|Rotator|MakeRotator (* _cameraroll (Utilities|Select :Index (Variables|WallRunning|GetWallRunSide) :NewEnumerator0 1.0 :NewEnumerator1 -1.0)) (.pitch _returnvalue_2) (.yaw _returnvalue_2))))))

(event Custom|BeginCrouch
  (bind _standingcapsulecapheight (Variables|Default|GetStandingCapsuleCapHeight))
  (bind _camera (Variables|Default|GetCamera))
  (bind _relativelocation (Variables|/Script/Engine.SceneComponent|GetRelativeLocation _camera))
  (bind _animtrack (Timeline|CrouchTimeline Play)
    (:Update
      (Components|Capsule|SetCapsuleHalfHeight (Variables|Collision|GetCapsuleComponent) (Math|Float|MapRangeClamped _animtrack 0.0 1.0 (/ _standingcapsulecapheight 1.5) _standingcapsulecapheight) true)
      (Transformation|SetRelativeLocation _camera (Math|Vector|MakeVector (.x _relativelocation) (.y _relativelocation) (Math|Float|MapRangeClamped _animtrack 0.0 1.0 25.0 (Variables|Default|GetStandingCameraZOffset))) false false))))

(event Custom|EndCrouch
  (bind _standingcapsulecapheight (Variables|Default|GetStandingCapsuleCapHeight))
  (bind _camera (Variables|Default|GetCamera))
  (bind _relativelocation (Variables|/Script/Engine.SceneComponent|GetRelativeLocation _camera))
  (bind _animtrack (Timeline|CrouchTimeline Reverse)
    (:Update
      (Components|Capsule|SetCapsuleHalfHeight (Variables|Collision|GetCapsuleComponent) (Math|Float|MapRangeClamped _animtrack 0.0 1.0 (/ _standingcapsulecapheight 1.5) _standingcapsulecapheight) true)
      (Transformation|SetRelativeLocation _camera (Math|Vector|MakeVector (.x _relativelocation) (.y _relativelocation) (Math|Float|MapRangeClamped _animtrack 0.0 1.0 25.0 (Variables|Default|GetStandingCameraZOffset))) false false))))

(event Custom|BeginSlide
  (Variables|Default|SetIsSliding true)
  (CallFunction|BeginSlideCameraTilt)
  (Timeline|SlideTimeline Play
    (:Update
      (Physics|AddForce (Variables|Character|GetCharacterMovement) (Sliding|CalculateFloorInfluence (.Normal (Collision|BreakHitResult (.HitResult (Utilities|Struct|BreakFindFloorResult (Variables|/Script/Engine.CharacterMovementComponent|GetCurrentFloor (Variables|Character|GetCharacterMovement))))))))
      (Utilities|FlowControl|Sequence
        (:then_0
          (if (> (Math|Vector|VectorLength (Transformation|GetVelocity)) (Variables|Movement|GetSprintSpeed))
            (Variables|/Script/Engine.MovementComponent|SetVelocity (Variables|Character|GetCharacterMovement) (* (Math|Vector|Normalize (Transformation|GetVelocity)) (Variables|Movement|GetSprintSpeed)))))
        (:then_1
          (if (not (Variables|Default|GetIsCrouchKeyDown))
            (CallFunction|ResolveMovementState)))
        (:then_2
          (if (< (Math|Vector|VectorLength (Transformation|GetVelocity)) (Variables|Movement|GetCrouchSpeed))
            (CallFunction|ResolveMovementState)))))))

(event EventBeginPlay
  (CallFunction|ResetJump (Variables|WallRunning|GetMaxJumps))
  (Class|MovementComponent|SetPlaneConstraintEnabled (Variables|Character|GetCharacterMovement) true)
  (CallFunction|InitializeMovementSpeed)
  (Variables|Default|SetStandingCameraZOffset (.z (Variables|/Script/Engine.SceneComponent|GetRelativeLocation (Variables|Default|GetCamera))))
  (Variables|Default|SetStandingCapsuleCapHeight (Components|Capsule|GetScaledCapsuleHalfHeight (Variables|Collision|GetCapsuleComponent)))
  (bind _returnvalue (UserInterface|CreateWidget "/Game/Blueprints/WBP_DebugUI.WBP_DebugUI_C"))
  (bind _output_get (Variables|Debug|SetDebugUI _returnvalue))
  (UserInterface|Viewport|AddtoViewport _output_get 0))

(event EventTick
  (params (DeltaSeconds :type Float%20%28single-precision%29))
  (WallRunning|ClampVelocity)
  (Utilities|SwitchMovementState
    (:Crouch
      (if (Movement|CanStand)
        (CallFunction|ResolveMovementState)))))

(event Input|KeyboardEvents|1
  (params (Key :type Key%20Structure :default "None"))
  (:Pressed
    (if (Variables|Debug|GetEnableDoubleJump)
      (Variables|Debug|SetEnableDoubleJump false)
      (else
        (Variables|Debug|SetEnableDoubleJump true)))))

(event Input|KeyboardEvents|2
  (params (Key :type Key%20Structure :default "None"))
  (:Pressed
    (bind _isa (Utilities|FlowControl|FlipFlop)
      (:A
        _)
      (:B
        _))
    (Widget|SetVisibility (Variables|Debug|GetDebugUI) (select _isa "Hidden" "Visible"))))

(event Custom|ResetJump
  (params (Jumps :type Integer))
  (Variables|WallRunning|SetJumpsLeft (Math|Integer|Clamp(Integer) Jumps 0 (Variables|WallRunning|GetMaxJumps))))

(event EventOnLanded
  (params (Hit :type Hit%20Result%20Structure%20%28by%20ref%29))
  (CallFunction|ResetJump (Variables|WallRunning|GetMaxJumps))
  (Variables|Movement|SetLocomotionState "NewEnumerator5"))

(event Input|ActionEvents|InputActionCrouch
  (params (Key :type Key%20Structure :default "None"))
  (:Pressed
    (Variables|Default|SetIsCrouchKeyDown true)
    (Utilities|SwitchLocomotionState
      (:Grounded
        (Utilities|SwitchMovementState
          (:Walk
            (CallFunction|SetMovementState "NewEnumerator7"))
          (:Sprint
            (CallFunction|SetMovementState "NewEnumerator8"))))))
  (:Released
    (Variables|Default|SetIsCrouchKeyDown false)
    (CallFunction|ResolveMovementState)))

(event Input|ActionEvents|InputActionSprint
  (params (Key :type Key%20Structure :default "None"))
  (:Pressed
    (Variables|Default|SetIsSprintKeyDown true)
    (Utilities|SwitchMovementState
      (:Walk
        _)
      (:Crouch
        _))
    (CallFunction|ResolveMovementState))
  (:Released
    (Variables|Default|SetIsSprintKeyDown false)
    (Utilities|SwitchMovementState
      (:Sprint
        (CallFunction|ResolveMovementState)))))

(event Input|ActionEvents|InputActionJump/WallRun
  (params (Key :type Key%20Structure :default "None"))
  (:Pressed
    (Utilities|SwitchLocomotionState
      (:Grounded
        (Utilities|SwitchMovementState
          (:Walk
            _)
          (:Sprint
            _)
          (:Crouch
            _)
          (:Slide
            (CallFunction|ResolveMovementState)))
        (Variables|Movement|SetLocomotionState "NewEnumerator6")
        (Utilities|ConsumeJump
          (:Consumed
            (Character|LaunchCharacter (WallRunning|FindLaunchVelocity) false true)
            (Utilities|OnWall
              (:true
                (CallFunction|EndWallRun "NewEnumerator1"))))))
      (:InAir
        (Variables|Default|SetIsWallRunKeyDown true)
        (Utilities|ConsumeJump
          (:Consumed
            (Character|LaunchCharacter (WallRunning|FindLaunchVelocity) false true))))))
  (:Released
    (Variables|Default|SetIsWallRunKeyDown false)
    (Character|StopJumping)))

(event Input|AxisEvents|InputAxisMoveForward
  (params (AxisValue :type Float%20%28single-precision%29))
  (bind _output_get (Variables|WallRunning|SetForwardAxis AxisValue))
  (Pawn|Input|AddMovementInput (Math|Vector|GetForwardVector (Variables|Collision|GetCapsuleComponent)) _output_get false))

(event Input|AxisEvents|InputAxisMoveRight
  (params (AxisValue :type Float%20%28single-precision%29))
  (bind _output_get (Variables|WallRunning|SetRightAxis AxisValue))
  (Pawn|Input|AddMovementInput (Math|Vector|GetRightVector (Variables|Collision|GetCapsuleComponent)) _output_get false))

(event Input|AxisEvents|InputAxisTurn
  (params (AxisValue :type Float%20%28single-precision%29))
  (Pawn|Input|AddControllerYawInput AxisValue))

(event Input|AxisEvents|InputAxisLookUp
  (params (AxisValue :type Float%20%28single-precision%29))
  (Pawn|Input|AddControllerPitchInput AxisValue))

(fn ConstructionScript)

(fn FindRunDirectionandSide
  (params (WallNormal :type Vector))
  (bind _output_get (LocalVariables|SetLocalSide (select (> (Math|Vector2D|DotProduct(2D) (Math|Conversions|ToVector2D(Vector) WallNormal) (Math|Conversions|ToVector2D(Vector) (Transformation|GetActorRightVector))) 0.0) "NewEnumerator0" "NewEnumerator1")))
  (return (Math|Vector|CrossProduct WallNormal (Utilities|Select :Index _output_get :NewEnumerator0 "0.000000, 0,-1.000000" :NewEnumerator1 "0,0.000000,1.000000")) (LocalVariables|GetLocalSide)))

(fn CanSurfacebeWallRan
  (params (SurfaceNormal :type Vector))
  (bind (_x _y _z) (Math|Vector|BreakVector SurfaceNormal))
  (if (< _z -0.05)
    (return false)
    (else
      (return (< (Class|KismetMathLibrary|DegAcos (Math|Vector|DotProduct (Math|Vector|Normalize (Math|Vector|MakeVector _x _y 0.0)) SurfaceNormal)) (Class|CharacterMovementComponent|GetWalkableFloorAngle (Variables|Character|GetCharacterMovement)))))))

(fn FindLaunchVelocity
  (Utilities|FlowControl|Sequence
    (:then_0
      (if (Variables|WallRunning|GetisWallRunning)
        (LocalVariables|SetLaunchDirection (Math|Vector|CrossProduct (Variables|WallRunning|GetWallRunDirection) (Utilities|Select :Index (Variables|WallRunning|GetWallRunSide) :NewEnumerator0 "0, 0,1.000000" :NewEnumerator1 "0.000000, 0,-1.000000")))
        (elif (AI|Components|NavMovement|IsFalling (Variables|Character|GetCharacterMovement))
          (LocalVariables|SetLaunchDirection (+ (* (Transformation|GetActorRightVector) (Variables|WallRunning|GetRightAxis)) (* (Transformation|GetActorForwardVector) (Variables|WallRunning|GetForwardAxis)))))))
    (:then_1
      (return (* (+ (LocalVariables|GetLaunchDirection) "0, 0,1.000000") (Variables|/Script/Engine.CharacterMovementComponent|GetJumpZVelocity (Variables|Character|GetCharacterMovement)))))))

(fn AreRequiredKeysDown
  (if (> (Variables|WallRunning|GetForwardAxis) 0.1)
    (return (Variables|Default|GetIsWallRunKeyDown))
    (else
      (return false))))

(fn GetHorizontalVelocity
  (return (Math|Conversions|ToVector2D(Vector) (Variables|/Script/Engine.MovementComponent|GetVelocity (Variables|Character|GetCharacterMovement)))))

(fn SetHorizontalVelocity
  (params (HorizontalVelocity :type Vector%202D%20Structure))
  (bind _charactermovement (Variables|Character|GetCharacterMovement))
  (Variables|/Script/Engine.MovementComponent|SetVelocity _charactermovement (Math|Vector|MakeVector (.x HorizontalVelocity) (.y HorizontalVelocity) (.z (Variables|/Script/Engine.MovementComponent|GetVelocity _charactermovement)))))

(fn UpdateWallRun
  (bind _returnvalue (Transformation|GetActorLocation))
  (bind _charactermovement (Variables|Character|GetCharacterMovement))
  (if (WallRunning|AreRequiredKeysDown)
    (bind (_outhit _returnvalue_2) (Collision|LineTraceByChannel _returnvalue (+ _returnvalue (* (Math|Vector|CrossProduct (Variables|WallRunning|GetWallRunDirection) (Utilities|Select :Index (Variables|WallRunning|GetWallRunSide) :NewEnumerator0 "0, 0,-1.000000" :NewEnumerator1 "0,0.000000,1.000000")) 1e+02)) "TraceTypeQuery1" false 0 "None"))
    (if _returnvalue_2
      (if (Utilities|Enum|Equal(Enum) (.Side (WallRunning|FindRunDirectionandSide (.ImpactNormal (Collision|BreakHitResult _outhit)))) (Variables|WallRunning|GetWallRunSide))
        (bind _output_get (Variables|WallRunning|SetWallRunDirection (.Direction (WallRunning|FindRunDirectionandSide (.ImpactNormal (Collision|BreakHitResult _outhit)))))) ; getting wall direction\nIE: wall has changed directions
        (Variables|/Script/Engine.MovementComponent|SetVelocity _charactermovement (Math|Vector|MakeVector (.x (* (* _output_get (Class|MovementComponent|GetModifiedMaxSpeed _charactermovement)) -1.0)) (.y (* (* _output_get (Class|MovementComponent|GetModifiedMaxSpeed _charactermovement)) -1.0)) 0.0)) ; update velocity to accomodate\nif walls change mid wall run
        (else
          (CallFunction|EndWallRun "NewEnumerator0")))
      (else
        (CallFunction|EndWallRun "NewEnumerator0")))
    (else
      (CallFunction|EndWallRun "NewEnumerator0"))))

(fn ClampVelocity
  (bind _returnvalue (Transformation|GetVelocity))
  (bind _maxvelocity (Variables|Movement|GetMaxVelocity))
  (bind (_x _y _z) (Math|Vector|BreakVector _returnvalue))
  (bind (_x_2 _y_2) (Math|Vector|BreakVector _returnvalue))
  (bind _returnvalue_2 (Math|Vector|MakeVector _x _y 0.0))
  (bind _returnvalue_3 (Math|Vector|ClampVectorSize _returnvalue_2 0.0 _maxvelocity))
  (bind (_x_3 _y_3) (Math|Vector|BreakVector _returnvalue_3))
  (if (AI|Components|NavMovement|IsFalling (Variables|Character|GetCharacterMovement))
    (if (not (Utilities|Enum|Equal(Enum) (Variables|Movement|GetLocomotionState) "NewEnumerator7"))
      (Variables|Movement|SetLocomotionState "NewEnumerator6")
      (if (> (Math|Vector|VectorLengthSquared (Math|Vector|MakeVector _x_2 _y_2 0.0)) (Variables|Movement|GetMaxVelocity))
        (Variables|/Script/Engine.MovementComponent|SetVelocity (Variables|Character|GetCharacterMovement) (Math|Vector|MakeVector _x_3 _y_3 _z))))))

(fn CanStand
  (bind _returnvalue (Transformation|GetActorLocation))
  (bind _capsulecomponent (Variables|Collision|GetCapsuleComponent))
  (bind _returnvalue_2 (Components|Capsule|GetScaledCapsuleHalfHeight _capsulecomponent))
  (bind _returnvalue_3 (- _returnvalue (Math|Vector|MakeVector 0.0 0.0 _returnvalue_2)))
  (if (Variables|Default|GetIsCrouchKeyDown)
    (return false)
    (else
      (bind _returnvalue_4 (Collision|LineTraceByChannel _returnvalue_3 (+ _returnvalue_3 (Math|Vector|MakeVector 0.0 0.0 (* (Variables|Default|GetStandingCapsuleCapHeight) 2.0))) "TraceTypeQuery1" false 0 "None"))
      (return (not _returnvalue_4)))))

(fn CanSprint
  (if (Variables|Default|GetIsSprintKeyDown)
    (return (Movement|CanStand))
    (else
      (return false))))

(fn ResolveMovementState
  (CallFunction|SetMovementState (select (Movement|CanSprint) "NewEnumerator5" (select (Movement|CanStand) "NewEnumerator1" "NewEnumerator7"))))

(fn SetMovementState
  (params (NewMovementState :type E_MovementState%20Enum :default "NewEnumerator1"))
  (if (Utilities|Enum|NotEqual(Enum) NewMovementState (Variables|Movement|GetMovementState))
    (LocalVariables|SetPrevMovementState (Variables|Movement|GetMovementState))
    (Variables|Movement|SetMovementState NewMovementState)
    (CallFunction|OnMovementStateChanged (LocalVariables|GetPrevMovementState))
    (Utilities|SwitchMovementState
      (:Walk
        (CallFunction|EndCrouch :!label _label))
      (:Sprint
        (goto _label))
      (:Crouch
        (CallFunction|BeginCrouch))
      (:Slide
        (Utilities|SwitchLocomotionState
          (:Grounded
            (CallFunction|BeginCrouch)
            (CallFunction|BeginSlide)))))))

(fn OnMovementStateChanged
  (params (PrevMovementState :type E_MovementState%20Enum :default "NewEnumerator1"))
  (bind _charactermovement (Variables|Character|GetCharacterMovement))
  (bind _charactermovement_2 (Variables|Character|GetCharacterMovement))
  (Utilities|FlowControl|Sequence
    (:then_0
      (Variables|Movement|SetTargetMovementSpeed (Utilities|Select :Index (Variables|Movement|GetMovementState) :NewEnumerator1 (Variables|Movement|GetWalkSpeed) :NewEnumerator5 (Variables|Movement|GetSprintSpeed) :NewEnumerator7 (Variables|Movement|GetCrouchSpeed) :NewEnumerator8 0.0))
      (CallFunction|ChangeMovementSpeed))
    (:then_1
      (switch Utilities|FlowControl|Switch|SwitchonE_MovementState PrevMovementState
        (:NewEnumerator8
          (Variables|/Script/Engine.CharacterMovementComponent|SetGroundFriction _charactermovement 8.0)
          (Variables|/Script/Engine.CharacterMovementComponent|SetBrakingDecelerationWalking _charactermovement 2048.0)
          (CallFunction|EndSlide))))
    (:then_2
      (Utilities|SwitchMovementState
        (:Slide
          (Variables|/Script/Engine.MovementComponent|SetVelocity _charactermovement_2 (* (Transformation|GetActorForwardVector) (Variables|Movement|GetSprintSpeed)))
          (Variables|/Script/Engine.CharacterMovementComponent|SetGroundFriction _charactermovement_2 0.0)
          (Variables|/Script/Engine.CharacterMovementComponent|SetBrakingDecelerationWalking _charactermovement_2 5e+02))))))

(fn InitializeMovementSpeed
  (bind _output_get (Variables|/Script/Engine.CharacterMovementComponent|SetMaxWalkSpeed (Variables|Character|GetCharacterMovement) (Variables|Movement|GetWalkSpeed)))
  (Variables|Movement|SetTargetMovementSpeed _output_get)
  (Variables|Movement|SetMaxVelocity (Variables|Movement|GetSprintSpeed)))

(fn CalculateFloorInfluence
  (params (FloorNormal :type Vector))
  (if (Math|Vector|Equal(Vector) FloorNormal (Math|Vector|VectorUp) 0.0001)
    (return "0.000000, 0, 0")
    (else
      (return (* (Math|Vector|Normalize (Math|Vector|CrossProduct FloorNormal (Math|Vector|CrossProduct FloorNormal (Math|Vector|VectorUp)))) (* (Math|Float|Clamp(Float) (- 1.0 (Math|Vector|DotProduct FloorNormal (Math|Vector|VectorUp)))) 1e+07))))))

(fn GetDebugInfo
  (bind _returnvalue (Transformation|GetVelocity))
  (return (Variables|Movement|GetLocomotionState) (Variables|Movement|GetMovementState) (Math|Vector2D|Vector2DLength (Math|Conversions|ToVector2D(Vector) _returnvalue)) (.Z (Math|Vector|BreakVector _returnvalue)) (Variables|Debug|GetEnableDoubleJump) (Variables|WallRunning|GetJumpsLeft)))