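; ACP_Health is a health component for BP_Player that starts at MaxHealth on BeginPlay and caches its owning player.
; UpdateHealth adds an amount capped at MaxHealth, while DamageHealth subtracts damage, clamping at zero and calling SetGamemodeState(true) when health runs out.
; GetHealth returns either the raw value or a fraction of MaxHealth.
; The LandDamageCalc event is an empty stub.
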(event Custom|LandDamageCalc)

(event EventBeginPlay
  (bind _asbp_player (Utilities|Casting|CastToBP_Player (Components|GetOwner)))
  (Variables|Default|SetPlayerRef _asbp_player)
  (Variables|Default|SetHealth (Variables|Default|GetMaxHealth)))

(fn GetHealth
  (params (FormatHealth :type Boolean))
  (if FormatHealth
    (return (/ (Variables|Default|GetHealth) (Variables|Default|GetMaxHealth)))
    (else
      (return (Variables|Default|GetHealth)))))

(fn UpdateHealth
  (params (Apply :type Float%20%28single-precision%29))
  (Variables|Default|SetHealth (select (> (+ Apply (Variables|Default|GetHealth)) (Variables|Default|GetMaxHealth)) (Variables|Default|GetMaxHealth) (+ Apply (Variables|Default|GetHealth)))))

(fn DamageHealth
  (params (Damage :type Float%20%28single-precision%29))
  (LocalVariables|SetUpdatedHealth (- (Variables|Default|GetHealth) Damage))
  (if (<= (LocalVariables|GetUpdatedHealth) 0.0)
    (Variables|Default|SetHealth 0.0)
    (CallFunction|SetGamemodeState true)
    (else
      (Variables|Default|SetHealth (LocalVariables|GetUpdatedHealth)))))