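; Zipline actor that carries a BP_Player along a straight cable once they touch it.
; Construction sets the spline and cable ends from CableEndLocation; BeginPlay stretches a trigger box along the spline.
; Overlap stores the player; Tick then repeatedly launches them along the spline's starting direction with slight lift.
; The ride stops when spline duration minus the player's closest input key reaches zero.
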(event OnComponentBeginOverlap(Box)
  (params (OverlappedComponent :type Primitive%20Component%20Object%20Reference) (OtherActor :type Actor%20Object%20Reference) (OtherComp :type Primitive%20Component%20Object%20Reference) (OtherBodyIndex :type Integer) (bFromSweep :type Boolean) (SweepResult :type Hit%20Result%20Structure%20%28by%20ref%29))
  (bind _spline (Variables|Default|GetSpline))
  (bind _asbp_player (Utilities|Casting|CastToBP_Player OtherActor))
  (bind _output_get (Variables|Default|SetPlayerRef _asbp_player))
  (Variables|Default|SetZiplineProgression 0.0)
  (Variables|Default|SetBeingUsed true)
  (Variables|Default|SetDistanceNeeded (- (Variables|/Script/Engine.SplineComponent|GetDuration _spline) (Class|SplineComponent|FindInputKeyClosesttoWorldLocation _spline (Transformation|GetActorLocation _output_get)))))

(event EventBeginPlay
  (bind _spline (Variables|Default|GetSpline))
  (bind _box (Variables|Default|GetBox))
  (Transformation|SetWorldLocation _box (.Origin (Collision|GetComponentBounds _spline)) false false)
  (Transformation|SetWorldRotation _box (Spline|GetRotationatDistanceAlongSpline _spline 1.0 "World") false false)
  (Components|Box|SetBoxExtent _box (Math|Vector|MakeVector (/ (Spline|GetSplineLength _spline) 2.0) 1e+01 1e+01) true))

(event EventTick
  (params (DeltaSeconds :type Float%20%28single-precision%29))
  (bind _spline (Variables|Default|GetSpline))
  (if (Variables|Default|GetBeingUsed)
    (Variables|Default|SetZiplineProgression (+ (Variables|Default|GetZiplineProgression) 0.005))
    (if (<= (Variables|Default|GetDistanceNeeded) 0.0)
      (Variables|Default|SetBeingUsed false)
      (else
        (Variables|Default|SetDistanceNeeded (- (Variables|/Script/Engine.SplineComponent|GetDuration _spline) (Class|SplineComponent|FindInputKeyClosesttoWorldLocation _spline (Transformation|GetActorLocation (Variables|Default|GetPlayerRef)))))
        (Character|LaunchCharacter (Variables|Default|GetPlayerRef) (+ (* (Math|Vector|GetForwardVector (Spline|GetRotationatDistanceAlongSpline (Variables|Default|GetSpline) 1.0 "World")) 1e+03) "0, 0,5.000000") true true)))))

(fn ConstructionScript
  (Spline|SetLocationatSplinePoint (Variables|Default|GetSpline) 1 (Variables|Default|GetCableEndLocation) "Local" true)
  (Variables|/Script/CableComponent.CableComponent|SetEndLocation (Variables|Default|GetCable) (Variables|Default|GetCableEndLocation)))