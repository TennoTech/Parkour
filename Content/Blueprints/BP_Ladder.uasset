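; BP_Ladder is a climbable ladder that BP_Player mounts automatically on overlapping its box.
; The construction script builds bottom, middle, connector and top mesh instances from the step count and sizes the box to fit.
; While mounted, gravity is off and a Timeline acts as a tick, turning forward input into vertical LaunchCharacter calls.
; Leaving the box launches the player forward, while descending onto floor pushes them backward, both restoring gravity.
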(event OnComponentBeginOverlap(Box)
  (params (OverlappedComponent :type Primitive%20Component%20Object%20Reference) (OtherActor :type Actor%20Object%20Reference) (OtherComp :type Primitive%20Component%20Object%20Reference) (OtherBodyIndex :type Integer) (bFromSweep :type Boolean) (SweepResult :type Hit%20Result%20Structure%20%28by%20ref%29))
  (bind _asbp_player (Utilities|Casting|CastToBP_Player OtherActor))
  (Variables|Default|SetIsInteractionCompleted false)
  (CallFunction|UseBPI true _asbp_player))

(event OnComponentEndOverlap(Box)
  (params (OverlappedComponent :type Primitive%20Component%20Object%20Reference) (OtherActor :type Actor%20Object%20Reference) (OtherComp :type Primitive%20Component%20Object%20Reference) (OtherBodyIndex :type Integer))
  (bind _asbp_player (Utilities|Casting|CastToBP_Player OtherActor))
  (Variables|Default|SetIsInteractionCompleted true)
  (CallFunction|UseBPI false _asbp_player))

(event Custom|OnLadder
  (params (OnLadder :type Boolean))
  (bind _playerref (Variables|Default|GetPlayerRef))
  (bind _playerref_2 (Variables|Default|GetPlayerRef))
  (bind _playerref_3 (Variables|Default|GetPlayerRef))
  (bind _playerref_4 (Variables|Default|GetPlayerRef))
  (bind _forwardaxis (Variables|/Game/Blueprints/Player/BP_Player.BP_Player_C|GetForwardAxis _playerref))
  (bind _charactermovement (Variables|/Script/Engine.Character|GetCharacterMovement _playerref_2))
  (if (Variables|Default|GetIsInteractionCompleted)
    (Variables|/Script/Engine.CharacterMovementComponent|SetGravityScale (Variables|/Script/Engine.Character|GetCharacterMovement (Variables|Default|GetPlayerRef)) 1.0)
    (Character|LaunchCharacter (Variables|Default|GetPlayerRef) (* (Transformation|GetActorForwardVector (Variables|Default|GetPlayerRef)) 1.5e+02) false false)
    (Timeline|Timeline_0 Stop
      (:Update
        (if (> (Math|Float|Absolute(Float) _forwardaxis) 0.1)
          (Character|LaunchCharacter (Variables|Default|GetPlayerRef) (* (Transformation|GetActorUpVector (Variables|Default|GetPlayerRef)) (* _forwardaxis 2.5e+02)) true true)
          (if (and (< (Variables|/Game/Blueprints/Player/BP_Player.BP_Player_C|GetForwardAxis _playerref_4) -0.1) (.bBlockingHit (Collision|BreakHitResult (.HitResult (Utilities|Struct|BreakFindFloorResult (Variables|/Script/Engine.CharacterMovementComponent|GetCurrentFloor (Variables|/Script/Engine.Character|GetCharacterMovement _playerref_4)))))))
            (Components|Movement|StopMovementImmediately (Variables|/Script/Engine.Character|GetCharacterMovement _playerref_3))
            (CallFunction|UseBPI false _playerref_3))
          (else
            (Components|Movement|StopMovementImmediately (Variables|/Script/Engine.Character|GetCharacterMovement (Variables|Default|GetPlayerRef)))))))
    (elif OnLadder
      (Variables|/Script/Engine.CharacterMovementComponent|SetGravityScale _charactermovement 0.0)
      (Timeline|Timeline_0 Play)
      (else
        (Variables|/Script/Engine.CharacterMovementComponent|SetGravityScale _charactermovement 1.0)
        (Character|LaunchCharacter (Variables|Default|GetPlayerRef) (* (Transformation|GetActorForwardVector (Variables|Default|GetPlayerRef)) -2.5e+02) false false)
        (Timeline|Timeline_0 Stop)))))

(event EventBeginPlay)

(event EventUseBPI
  (params (IsUsing :type Boolean) (Player :type BP%20Player%20Object%20Reference))
  (bind _output_get (Variables|Default|SetPlayerRef Player))
  (Default|SetOverlayState _output_get (select IsUsing (CallFunction|GetInteractableType) "NewEnumerator3") self)
  (CallFunction|OnLadder IsUsing)
  (if IsUsing
    (Variables|/Game/Blueprints/Player/BP_Player.BP_Player_C|SetTransitionInteractState (Variables|Default|GetPlayerRef) true)
    (Variables|Default|SetIsInteractionCompleted false)))

(fn ConstructionScript
  (bind _ladderstep (Variables|Default|GetLadderStep))
  (bind _returnvalue (- _ladderstep 1))
  (|CallParentFunction)
  (for _index (range 0 _returnvalue)
    (if (== _index 0)
      (Components|InstancedStaticMesh|AddInstance (Variables|Default|GetLadderBottom) (Math|Transform|MakeTransform (Math|Vector|MakeVector 0.0 0.0 (* _index (Variables|Default|GetLadderHeight))) "0, 0, 0" "1,1,1"))
      (elif (== _index _returnvalue)
        (Components|InstancedStaticMesh|AddInstance (Variables|Default|GetLadderTop) (Math|Transform|MakeTransform (Math|Vector|MakeVector 0.0 0.0 (* _index (Variables|Default|GetLadderHeight))) "0, 0, 0" "1,1,1"))
        (Transformation|SetRelativeLocation (Variables|Default|GetBox) (Math|Vector|MakeVector 0.0 1e+01 (- (Math|Conversions|ToFloat(Integer) (* (Variables|Default|GetLadderStep) 20)) 2e+01)) false false)
        (Components|Box|SetBoxExtent (Variables|Default|GetBox) (Math|Vector|MakeVector 3e+01 1e+01 (Math|Conversions|ToFloat(Integer) (* (Variables|Default|GetLadderStep) 20))) true)
        (elif (== (Math|Integer|%(Integer) _index (Variables|Default|GetConnectRate)) 0)
          (Components|InstancedStaticMesh|AddInstance (Variables|Default|GetLadderConnect) (Math|Transform|MakeTransform (Math|Vector|MakeVector 0.0 0.0 (* _index (Variables|Default|GetLadderHeight))) "0, 0, 0" "1,1,1"))
          (else
            (Components|InstancedStaticMesh|AddInstance (Variables|Default|GetLadderMiddle) (Math|Transform|MakeTransform (Math|Vector|MakeVector 0.0 0.0 (* _index (Variables|Default|GetLadderHeight))) "0, 0, 0" "1,1,1"))))))))

(fn GetInteractableType
  (return "NewEnumerator1"))